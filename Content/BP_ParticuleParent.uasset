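; Parent Blueprint for physics-driven element particles (Oxygen, Carbone, Hydrogen, Helium) that react to one another.
; Element type sets material and Niagara effect at construction, and a temperature value at BeginPlay, which is debug-printed.
; Each Tick, a stationary sphere trace finds another particle: Hydrogen converts Oxygen to Hydrogen, swapping only type and effect.
; Otherwise, the detected particle is pushed up if hotter, down if colder.
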(event `self.ReceiveTick`
  (params (DeltaSeconds :type "Float (single-precision)"))
  (bind _returnvalue (`SceneComponent.K2_GetComponentLocation` (`self.Particle`)))
  (`|ExecutionSequence`
    (:`then_0`
      (bind (_outhit _returnvalue_2) (`KismetSystemLibrary.SphereTraceSingle` _returnvalue _returnvalue 500.0 "TraceTypeQuery1"))
      (if _returnvalue_2
        (bind _asbp_particule_parent (cast `/Game/BP_ParticuleParent` (`.HitActor` (`GameplayStatics.BreakHitResult` _outhit))))
        (if (and (`|EnumEquality` (`/Game/BP_ParticuleParent.E_Type` _asbp_particule_parent) "NewEnumerator3") (`|EnumEquality` (`self.E_Type`) "NewEnumerator0"))
          (set `self.E_Type` "NewEnumerator3")
          (`NiagaraComponent.SetAsset` (`self.NS_Oxygen`) "/Game/NS_Hydrogene.NS_Hydrogene" true)
          (elif (> (`/Game/BP_ParticuleParent.TempOfTheOther` _asbp_particule_parent) (`self.TempOfTheOther`))
            (`PrimitiveComponent.AddForce` (`/Game/BP_ParticuleParent.Particle` _asbp_particule_parent) (0.0 0.0 10000.0) "None" false)
            (elif (not (== (`/Game/BP_ParticuleParent.TempOfTheOther` _asbp_particule_parent) (`self.TempOfTheOther`)))
              (`PrimitiveComponent.AddForce` (`/Game/BP_ParticuleParent.Particle` _asbp_particule_parent) (0.0 0.0 -5000.0) "None" false))))))))

(event `self.ReceiveBeginPlay`
  (bind _output_get (set `self.TempOfTheOther` (select `/Game/E_TypeOfParticule` (`self.E_Type`) :`NewEnumerator0` 10.0 :`NewEnumerator1` 20.0 :`NewEnumerator3` 30.0 :`NewEnumerator4` 40.0)))
  (`KismetSystemLibrary.PrintString` (`KismetStringLibrary.Concat_StrStr` (`|GetEnumeratorNameAsString` (`self.E_Type`)) "" (`KismetStringLibrary.Conv_DoubleToString` _output_get)) true true (struct :`G` 0.66 :`B` 1.0 :`A` 1.0) 200.0))

(fn `UserConstructionScript`
  (`PrimitiveComponent.SetMaterial` (`self.Particle`) 0 (select `/Game/E_TypeOfParticule` (`self.E_Type`) :`NewEnumerator0` "/Game/LevelPrototyping/Materials/MI_Solid_Blue.MI_Solid_Blue" :`NewEnumerator1` "/Game/StarterContent/Blueprints/Assets/M_LightStage_Skybox_Black.M_LightStage_Skybox_Black" :`NewEnumerator3` "/Game/StarterContent/Materials/M_Metal_Copper.M_Metal_Copper" :`NewEnumerator4` "/Game/StarterContent/Materials/M_Glass.M_Glass" :!type "MaterialInterface Object Reference"))
  (`NiagaraComponent.SetAsset` (`self.NS_Oxygen`) (select `/Game/E_TypeOfParticule` (`self.E_Type`) :`NewEnumerator0` "/Game/NS_Oxygen.NS_Oxygen" :`NewEnumerator1` "/Game/NS_Carbone.NS_Carbone" :`NewEnumerator3` "/Game/NS_Hydrogene.NS_Hydrogene" :`NewEnumerator4` "/Game/NS_Helium.NS_Helium" :!type "NiagaraSystem Object Reference") true))